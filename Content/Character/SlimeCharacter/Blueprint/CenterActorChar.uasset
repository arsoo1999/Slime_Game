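; CenterActorChar is a pivot actor that turns the female third-person player character around a center point.
; On BeginPlay it attaches the player pawn to itself, so rotating the actor carries the character along.
; RotateCenter prints the swipe direction, then plays a timeline that sets yaw from RotateZ plus the curve value selected by the character's SelectRotate.
; When the timeline finishes, it sets EndAnim on the character.
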(event Custom|Rotate%20Center
  (Development|PrintString (Utilities|String|EnumtoString (Variables|/Game/Character/SlimeCharacter/Blueprint/ThirdPersonCharacter_Female.ThirdPersonCharacter_Female_C|GetSwipeDetection (stale EventBeginPlay _asthird_person_character_female))))
  (bind (_direction _rotate _rotate_) (Timeline|Rotate PlayFromStart)
    (:Update
      (Transformation|SetActorRotation (Math|Interpolation|RInterpTo (Transformation|GetActorRotation) (Math|Rotator|MakeRotator 0.0 0.0 (+ (Variables|Default|GetRotateZ) (Utilities|Select :Index (Variables|/Game/Character/SlimeCharacter/Blueprint/ThirdPersonCharacter_Female.ThirdPersonCharacter_Female_C|GetSelectRotate (stale EventBeginPlay _asthird_person_character_female)) :Option%200 _rotate :Option%201 _rotate_))) (Utilities|Time|GetWorldDeltaSeconds) 0.0)))
    (:Finished
      (Variables|/Game/Character/SlimeCharacter/Blueprint/ThirdPersonCharacter_Female.ThirdPersonCharacter_Female_C|SetEndAnim (stale EventBeginPlay _asthird_person_character_female) true))))

(event EventBeginPlay
  (bind _asthird_person_character_female (Utilities|Casting|CastToThirdPersonCharacter_Female (Game|Player|GetPlayerPawn 0)))
  (Transformation|AttachActorToActor _asthird_person_character_female self "None" "KeepRelative" "KeepRelative" "KeepRelative" true))

(fn ConstructionScript)